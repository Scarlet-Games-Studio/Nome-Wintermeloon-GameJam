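; BP_GrandmaNPC is a grandma NPC that shows its dialogue on screen, one line per Talk event.
; Talk increments TalkIndex, creates and caches a WB_Dialogue widget if none is valid, then writes that Dialogue array entry into its TalkText.
; The index has no effective bounds check, as the length comparison is left unconnected and the branch is always true.
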(event `/Game/J64d/InventoryComponent/NPCInteract/BPI_Dialogue.Talk`
  (`/Engine/EditorBlueprintResources/StandardMacros.IncrementInt` (`self.TalkIndex`)
    (:`  `
      (if true
        (`self.UI`
          (:`then`
            _)
          (:`else`
            (bind _returnvalue (`|CreateWidget` "/Game/J64d/InventoryComponent/NPCInteract/WB_Dialogue.WB_Dialogue_C" (`GameplayStatics.GetPlayerController` 0)))
            (bind _output_get (set `self.UI` _returnvalue))
            (`UserWidget.AddToViewport` (`self.UI`) 0)
            (`UserWidget.AddToViewport` _output_get 0)))
        (`TextBlock.SetText` (`/Game/J64d/InventoryComponent/NPCInteract/WB_Dialogue.TalkText` (`self.UI`)) (`KismetTextLibrary.Conv_StringToText` (`|GetArrayItem` (`self.Dialogue`) (`self.TalkIndex`))))))))

(fn `UserConstructionScript`)