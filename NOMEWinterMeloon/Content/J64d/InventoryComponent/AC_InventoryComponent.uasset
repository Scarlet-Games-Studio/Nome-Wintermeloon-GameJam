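; Inventory actor component that shows and hides the inventory widget for the player.
; Showing creates a new inventory widget for the first player controller if it is local, adds it to the viewport and updates it with the component's inventory data.
; Hiding removes the stored widget from its parent when it is valid.
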(fn `F_HideInventory`
  (`/Engine/EditorBlueprintResources/StandardMacros.IsValid` (`self.WB_Inventory`)
    (:`Is Valid`
      (`Widget.RemoveFromParent` (`self.WB_Inventory`)))))

(fn `F_ShowInventory`
  (bind _returnvalue (`GameplayStatics.GetPlayerController` 0))
  (if (`Controller.IsLocalPlayerController` _returnvalue)
    (bind _returnvalue_2 (`|GenericCreateObject` _returnvalue "/Game/J64d/InventoryComponent/WB_Inventory.WB_Inventory_C"))
    (bind _output_get (set `self.WB_Inventory` _returnvalue_2))
    (`UserWidget.AddToViewport` _output_get 0)
    (`/Game/J64d/InventoryComponent/WB_Inventory.F Update` _returnvalue_2 (`self.Inventory`))))